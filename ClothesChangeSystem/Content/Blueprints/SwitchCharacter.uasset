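; Modular character customization preview that swaps clothing, hair, beard and sunglasses and rotates by click-dragging on its capsule.
; The selected part picks a material array, and material changes also equip that part's mesh or revert it to default or empty.
; Parts follow Head via master pose, while a selected montage plays on each component and replays on completion.
; SavePartsData stores meshes and materials in PartsData, with beard and sunglasses materials crossed.
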(event OnClicked(CapsuleComponent)
  (params (TouchedComponent :type Primitive%20Component%20Object%20Reference) (ButtonPressed :type Key%20Structure :default "None"))
  ;[1 1 1] MouseEvent
  (Variables|Default|SetIsMouseClick true)
  (bind _returnvalue (Class|WidgetLayoutLibrary|GetMousePositiononViewport))
  (Variables|Default|SetPreMousePosition _returnvalue))

(event Custom|ChangeMaterial_Null
  ;[1 1 1] ChangeMaterial
  (switch Utilities|FlowControl|Switch|SwitchonE_Parts (Variables|Default|GetCurrentPart)
    (:NewEnumerator0
      (CallFunction|AddSunGlasses false))
    (:NewEnumerator1
      (CallFunction|AddPants false))
    (:NewEnumerator2
      (CallFunction|AddJacket "/Game/Assets/SCK_Casual01/Models/MESH_T_01.MESH_T_01" false))
    (:NewEnumerator3
      (CallFunction|AddJacket "/Game/Assets/SCK_Casual01/Models/MESH_T_03.MESH_T_03" false))
    (:NewEnumerator4
      (CallFunction|AddHair "/Game/Assets/SCK_Casual01/Models/MESH_A_02.MESH_A_02" false))
    (:NewEnumerator5
      (CallFunction|AddHair "/Game/Assets/SCK_Casual01/Models/MESH_A_03.MESH_A_03" false))
    (:NewEnumerator6
      (CallFunction|AddBeard false))))

(event Custom|LeftMouseButtonReleased
  ;[1 1 1] MouseEvent
  (Variables|Default|SetIsMouseClick false)
  (Variables|Default|SetDefaultRotation (Transformation|GetWorldRotation (Variables|Default|GetCapsuleComponent))))

(event Custom|AddJacket
  (params (NewMesh :type Skeletal%20Mesh%20Object%20Reference) (State :type Boolean))
  (bind _torso (Variables|Default|GetTorso))
  ;[1 1 1] AddClothes
  ;;[1 1 1] AddJacket
  (if State
    (Class|SkinnedMeshComponent|SetSkeletalMesh _torso NewMesh true)
    (else
      (Class|SkinnedMeshComponent|SetSkeletalMesh _torso "/Game/Assets/SCK_Casual01/Models/MESH_T_00.MESH_T_00" true)
      (Rendering|Material|SetMaterial _torso 0 "/Game/Assets/SCK_Casual01/Materials/Master_Materials/MAT_T_00.MAT_T_00"))))

(event Custom|UpdataCurrentMaterial
  (params (ChangePart :type E_Parts%20Enum :default "NewEnumerator0"))
  ;[1 1 1] UpdataCurrentMaterial
  (bind _output_get (Variables|Default|SetCurrentPart ChangePart))
  (switch Utilities|FlowControl|Switch|SwitchonE_Parts _output_get
    (:NewEnumerator0
      (Variables|Default|SetCurrentMaterial (Variables|Default|GetSunGlassesM)))
    (:NewEnumerator1
      (Variables|Default|SetCurrentMaterial (Variables|Default|GetpantsM)))
    (:NewEnumerator2
      (Variables|Default|SetCurrentMaterial (Variables|Default|GetJacketM1)))
    (:NewEnumerator3
      (Variables|Default|SetCurrentMaterial (Variables|Default|GetJacketM2)))
    (:NewEnumerator4
      (Variables|Default|SetCurrentMaterial (Variables|Default|GetHairM1)))
    (:NewEnumerator5
      (Variables|Default|SetCurrentMaterial (Variables|Default|GetHairM2)))
    (:NewEnumerator6
      (Variables|Default|SetCurrentMaterial (Variables|Default|GetBeardM)))))

(event Custom|SavePartsData
  (bind _sunglasses (Variables|Default|GetSunGlasses))
  (bind _torso (Variables|Default|GetTorso))
  (bind _legs (Variables|Default|GetLegs))
  (bind _hair (Variables|Default|GetHair))
  (bind _beard (Variables|Default|GetBeard))
  ;[1 1 1] SavePartsData
  (Utilities|Struct|SetmembersinS_PartsData (Variables|Default|GetPartsData) (Variables|/Script/Engine.SkinnedMeshComponent|GetSkeletalMesh _torso) (Variables|/Script/Engine.SkinnedMeshComponent|GetSkeletalMesh _legs) (Variables|/Script/Engine.SkinnedMeshComponent|GetSkeletalMesh _hair) (Variables|/Script/Engine.SkinnedMeshComponent|GetSkeletalMesh _sunglasses) (Variables|/Script/Engine.SkinnedMeshComponent|GetSkeletalMesh _beard) (Utilities|Array|Get(acopy) (Rendering|Material|GetMaterials _torso)) (Utilities|Array|Get(acopy) (Rendering|Material|GetMaterials _legs)) (Utilities|Array|Get(acopy) (Rendering|Material|GetMaterials _hair)) (Utilities|Array|Get(acopy) (Rendering|Material|GetMaterials _beard)) (Utilities|Array|Get(acopy) (Rendering|Material|GetMaterials _sunglasses))))

(event Custom|AddPants
  (params (State :type Boolean))
  (bind _legs (Variables|Default|GetLegs))
  ;[1 1 1] AddClothes
  ;;[1 1 1] AddPants
  (if State
    (Class|SkinnedMeshComponent|SetSkeletalMesh _legs "/Game/Assets/SCK_Casual01/Models/MESH_L_01.MESH_L_01" true)
    (else
      (Class|SkinnedMeshComponent|SetSkeletalMesh _legs "/Game/Assets/SCK_Casual01/Models/MESH_L_00.MESH_L_00" true)
      (Rendering|Material|SetMaterial _legs 0 "/Game/Assets/SCK_Casual01/Materials/Master_Materials/MAT_L_00.MAT_L_00"))))

(event Custom|AddBeard
  (params (State :type Boolean))
  (bind _beard (Variables|Default|GetBeard))
  ;[1 1 1] AddClothes
  ;;[1 1 1] AddBeard
  (if State
    (Class|SkinnedMeshComponent|SetSkeletalMesh _beard "/Game/Assets/SCK_Casual01/Models/MESH_A_04.MESH_A_04" true)
    (else
      (Class|SkinnedMeshComponent|SetSkeletalMesh _beard 0 true))))

(event Custom|AddHair
  (params (NewMesh :type Skeletal%20Mesh%20Object%20Reference) (State :type Boolean))
  (bind _hair (Variables|Default|GetHair))
  ;[1 1 1] AddClothes
  ;;[1 1 1] AddHair
  (if State
    (Class|SkinnedMeshComponent|SetSkeletalMesh _hair NewMesh true)
    (else
      (Class|SkinnedMeshComponent|SetSkeletalMesh _hair 0 true))))

(event Custom|ChangeActions
  (params (Num :type Integer))
  ;[1 1 1] ChangeActions
  (bind _output_get (Variables|Default|SetActionNum Num))
  (Animation|Montage|PlayMontage (Variables|Default|GetHead) (Utilities|Array|Get(acopy) (Variables|Default|GetAnimSequences) _output_get)
    (:then
      (Animation|Montage|PlayMontage (Variables|Default|GetLegs) (Utilities|Array|Get(acopy) (Variables|Default|GetAnimSequences) _output_get)
        (:then
          (Animation|Montage|PlayMontage (Variables|Default|GetHair) (Utilities|Array|Get(acopy) (Variables|Default|GetAnimSequences) _output_get)
            (:then
              (Animation|Montage|PlayMontage (Variables|Default|GetHands) (Utilities|Array|Get(acopy) (Variables|Default|GetAnimSequences) _output_get)
                (:then
                  (Animation|Montage|PlayMontage (Variables|Default|GetBeard) (Utilities|Array|Get(acopy) (Variables|Default|GetAnimSequences) _output_get)
                    (:then
                      (Animation|Montage|PlayMontage (Variables|Default|GetSunGlasses) (Utilities|Array|Get(acopy) (Variables|Default|GetAnimSequences) _output_get)
                        (:then
                          (Animation|Montage|PlayMontage (Variables|Default|GetTorso) (Utilities|Array|Get(acopy) (Variables|Default|GetAnimSequences) _output_get)
                            (:OnCompleted
                              (CallFunction|ChangeActions (Variables|Default|GetActionNum)))))
                        (:OnCompleted
                          (CallFunction|ChangeActions (Variables|Default|GetActionNum)))))
                    (:OnCompleted
                      (CallFunction|ChangeActions (Variables|Default|GetActionNum)))))
                (:OnCompleted
                  (CallFunction|ChangeActions (Variables|Default|GetActionNum)))))
            (:OnCompleted
              (CallFunction|ChangeActions (Variables|Default|GetActionNum)))))
        (:OnCompleted
          (CallFunction|ChangeActions (Variables|Default|GetActionNum)))))
    (:OnCompleted
      (CallFunction|ChangeActions (Variables|Default|GetActionNum)))))

(event Custom|AddSunGlasses
  (params (State :type Boolean))
  (bind _sunglasses (Variables|Default|GetSunGlasses))
  ;[1 1 1] AddClothes
  ;;[1 1 1] AddSunGlasses
  (if State
    (Class|SkinnedMeshComponent|SetSkeletalMesh _sunglasses "/Game/Assets/SCK_Casual01/Models/MESH_A_01.MESH_A_01" true)
    (else
      (Class|SkinnedMeshComponent|SetSkeletalMesh _sunglasses 0 true))))

(event Custom|ChangeMaterial
  (params (Num :type Integer))
  (bind _currentmaterial (Variables|Default|GetCurrentMaterial))
  (bind _torso (Variables|Default|GetTorso))
  (bind _hair (Variables|Default|GetHair))
  (bind _output (Utilities|Array|Get(acopy) _currentmaterial Num))
  ;[1 1 1] ChangeMaterial
  (switch Utilities|FlowControl|Switch|SwitchonE_Parts (Variables|Default|GetCurrentPart)
    (:NewEnumerator0
      (CallFunction|AddSunGlasses true)
      (Rendering|Material|SetMaterial (Variables|Default|GetSunGlasses) 0 _output))
    (:NewEnumerator1
      (CallFunction|AddPants true)
      (Rendering|Material|SetMaterial (Variables|Default|GetLegs) 0 _output))
    (:NewEnumerator2
      (CallFunction|AddJacket "/Game/Assets/SCK_Casual01/Models/MESH_T_01.MESH_T_01" true)
      (Rendering|Material|SetMaterial _torso 0 _output))
    (:NewEnumerator3
      (CallFunction|AddJacket "/Game/Assets/SCK_Casual01/Models/MESH_T_03.MESH_T_03" true)
      (Rendering|Material|SetMaterial _torso 0 _output))
    (:NewEnumerator4
      (CallFunction|AddHair "/Game/Assets/SCK_Casual01/Models/MESH_A_02.MESH_A_02" true)
      (Rendering|Material|SetMaterial _hair 0 _output))
    (:NewEnumerator5
      (CallFunction|AddHair "/Game/Assets/SCK_Casual01/Models/MESH_A_03.MESH_A_03" true)
      (Rendering|Material|SetMaterial _hair 0 _output))
    (:NewEnumerator6
      (CallFunction|AddBeard true)
      (Rendering|Material|SetMaterial (Variables|Default|GetBeard) 0 _output))))

(event EventBeginPlay
  ;[1 1 1] EnvetBeginPlay
  (Variables|Default|SetCurrentMaterial (Variables|Default|GetHairM2)))

(event EventTick
  (params (DeltaSeconds :type Float%20%28single-precision%29))
  ;[1 1 1] MouseChangePlayerRotation
  (if (Variables|Default|GetIsMouseClick)
    (bind _returnvalue (Class|WidgetLayoutLibrary|GetMousePositiononViewport))
    (Variables|Default|SetCurrentMousePosition _returnvalue)
    (Transformation|SetWorldRotation (Variables|Default|GetCapsuleComponent) (Math|Rotator|MakeRotator 0.0 0.0 (+ (/ (.x (- (Variables|Default|GetPreMousePosition) (Variables|Default|GetCurrentMousePosition))) 3.0) (.yaw (Variables|Default|GetDefaultRotation)))) false false)))

(fn ConstructionScript
  ;[1 1 1] SetMasterPoseComponent
  (Class|SkinnedMeshComponent|SetMasterPoseComponent (Variables|Default|GetLegs) (Variables|Default|GetHead) false))