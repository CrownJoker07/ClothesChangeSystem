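; Player controller for a character and clothes switching screen.
; On BeginPlay it caches the MyGameInstance, adds the WB_SwitchClothes widget to the viewport, shows the mouse cursor and finds the SwitchCharacter actor in the level.
; On left mouse button release it calls that actor's LeftMouseButtonReleased, but only while the actor's IsMouseClick flag is set.
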(event EventBeginPlay
  (bind _asmy_game_instance (Utilities|Casting|CastToMyGameInstance (Game|GetGameInstance)))
  (Variables|Default|SetMyGameInstanceREF _asmy_game_instance)
  (bind _returnvalue (UserInterface|CreateWidget "/Game/Blueprints/UMG/WB_SwitchClothes.WB_SwitchClothes_C"))
  (UserInterface|Viewport|AddtoViewport _returnvalue 0)
  (Variables|Default|SetbShowMouseCursor true)
  (bind _returnvalue_2 (Actor|GetActorOfClass "/Game/Blueprints/SwitchCharacter.SwitchCharacter_C"))
  (Variables|Default|SetSwitchCharacter _returnvalue_2))

(event EventTick
  (params (DeltaSeconds :type Float%20%28single-precision%29)))

(event Input|MouseEvents|LeftMouseButton
  (params (Key :type Key%20Structure :default "None"))
  (bind _switchcharacter (Variables|Default|GetSwitchCharacter))
  (:Released
    (if (Variables|/Game/Blueprints/SwitchCharacter.SwitchCharacter_C|GetIsMouseClick _switchcharacter)
      (Default|LeftMouseButtonReleased _switchcharacter))))

(fn ConstructionScript)